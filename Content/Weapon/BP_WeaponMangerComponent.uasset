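; Player weapon manager component that spawns the equipped weapon, attaches it to the character's hand socket and handles shooting, reloading and the magazine HUD.
; Shooting requires aiming, ammo and no active reload, with a delay that sets fire rate and repeats shots for automatic weapons.
; Bullets spawn at the muzzle, rotated toward a shoulder-camera trace hit that ignores NO_SHOT actors.
; Ammo changes update the weapon struct and magazine widget.
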(event Custom|ShootDelay
  (bind _equipedweapon (Variables|Default|GetEquipedWeapon))
  (bind _weaponstruct (Variables|/Game/Weapon/BP_MasterWeapon.BP_MasterWeapon_C|GetWeaponStruct _equipedweapon))
  (Utilities|FlowControl|Delay (.shootspeed _weaponstruct))
  (Variables|Default|SetCanShoot true)
  (if (not (.singleshoot _weaponstruct))
    (CallFunction|Shoot)))

(event EventBeginPlay
  (CallFunction|SetPlayerRef)
  (CallFunction|SpawnEquipedWeapon)
  (CallFunction|AttachEquipedtoHandSocket "right_hand_socket")
  (CallFunction|AddWidgets))

(event EventTick
  (params (DeltaSeconds :type Float%20%28single-precision%29)))

(event Input|ActionEvents|InputActionShoot
  (params (Key :type Key%20Structure :default "None"))
  (:Pressed
    (CallFunction|StartShooting))
  (:Released
    (CallFunction|StopShooting)))

(event Input|ActionEvents|InputActionReload
  (params (Key :type Key%20Structure :default "None"))
  (:Pressed
    (Variables|Default|SetIsReloading true)
    (Utilities|FlowControl|Delay (.reloadtime (Variables|/Game/Weapon/BP_MasterWeapon.BP_MasterWeapon_C|GetWeaponStruct (Variables|Default|GetEquipedWeapon))))
    (CallFunction|ReloadEquipedWeapon)))

(fn GetEquipedWeapon
  (return (Variables|Default|GetEquipedWeapon)))

(fn AttachEquipedtoHandSocket
  (params (HandSocket :type Name))
  (Transformation|AttachComponentToComponent (Variables|Default|GetEquipedWeapon) (Variables|/Script/Engine.Character|GetMesh (Variables|Default|GetPlayerRef)) HandSocket "SnapToTarget" "SnapToTarget" "KeepRelative" true))

(fn SetPlayerRef
  (bind _asthird_person_character (Utilities|Casting|CastToThirdPersonCharacter (Game|GetPlayerCharacter 0)))
  (Variables|Default|SetPlayerRef _asthird_person_character))

(fn SpawnEquipedWeapon
  (bind _returnvalue (Game|SpawnActorfromClass (Variables|Default|GetWeapon) (Transformation|GetActorTransform (Variables|Default|GetPlayerRef)) "Undefined" 0 0))
  (Variables|Default|SetEquipedWeapon _returnvalue)
  (Development|PrintString "Weapon spawned"))

(fn GetEquipedWeaponLeftHandPosition
  (return (Variables|/Game/Weapon/BP_MasterWeapon.BP_MasterWeapon_C|GetLeftHandPosition (Variables|Default|GetEquipedWeapon))))

(fn Shoot
  (bind _hasammunition (CallFunction|HasAmmunition))
  (if (Math|Boolean|ANDBoolean _hasammunition (Variables|/Game/ThirdPersonBP/Blueprints/ThirdPersonCharacter.ThirdPersonCharacter_C|GetIsAiming (Variables|Default|GetPlayerRef)) (Variables|Default|GetCanShoot) (Variables|Default|GetIsShooting) (not (Variables|Default|GetIsReloading)))
    (Variables|Default|SetCanShoot false)
    (CallFunction|UseAmmunition)
    (CallFunction|SpawnBullet)
    (CallFunction|ShootDelay)))

(fn GetShootTargetPosition
  (bind _playerref (Variables|Default|GetPlayerRef))
  (bind _shouldercamera (Variables|/Game/ThirdPersonBP/Blueprints/ThirdPersonCharacter.ThirdPersonCharacter_C|GetShoulderCamera _playerref))
  (bind _returnvalue (Transformation|GetWorldLocation _shouldercamera))
  (bind _outactors (Actor|GetAllActorswithTag "NO_SHOT"))
  (bind _outhit (Collision|LineTraceByChannel _returnvalue (+ _returnvalue (* (Math|Vector|GetForwardVector (Transformation|GetWorldRotation _shouldercamera)) (Variables|Default|GetShootDistance))) "TraceTypeQuery3" false _outactors "None"))
  (return (.Location (Collision|BreakHitResult _outhit))))

(fn SpawnBullet
  (bind _equipedweapon (Variables|Default|GetEquipedWeapon))
  (bind _shootposition (Variables|/Game/Weapon/BP_MasterWeapon.BP_MasterWeapon_C|GetShootPosition _equipedweapon))
  (bind _hitposition (CallFunction|GetShootTargetPosition))
  (Game|SpawnActorfromClass "/Game/Rifles/u-rifle/BasicBullet.BasicBullet_C" (Transformation|GetWorldTransform _shootposition) "Undefined" 0 (Math|Rotator|FindLookatRotation (Transformation|GetWorldLocation _shootposition) _hitposition) (.damage (Variables|/Game/Weapon/BP_MasterWeapon.BP_MasterWeapon_C|GetWeaponStruct _equipedweapon)) 0))

(fn StopShooting
  (Variables|Default|SetIsShooting false))

(fn StartShooting
  (Variables|Default|SetIsShooting true)
  (CallFunction|Shoot))

(fn UseAmmunition
  (CallFunction|SetAmmunition (- (.ammoinmagazine (Variables|/Game/Weapon/BP_MasterWeapon.BP_MasterWeapon_C|GetWeaponStruct (Variables|Default|GetEquipedWeapon))) 1)))

(fn HasAmmunition
  (return (> (.ammoinmagazine (Variables|/Game/Weapon/BP_MasterWeapon.BP_MasterWeapon_C|GetWeaponStruct (Variables|Default|GetEquipedWeapon))) 0)))

(fn ReloadEquipedWeapon
  (CallFunction|SetAmmunition (.magazinesize (Variables|/Game/Weapon/BP_MasterWeapon.BP_MasterWeapon_C|GetWeaponStruct (Variables|Default|GetEquipedWeapon))))
  (Variables|Default|SetIsReloading false))

(fn AddWidgets
  (bind _returnvalue (UserInterface|CreateWidget "/Game/UI/Magazine/Magazine_Widget.Magazine_Widget_C"))
  (UserInterface|Viewport|AddtoViewport _returnvalue 0)
  (bind _output_get (Variables|Default|SetMagazineWidget _returnvalue))
  (Default|SetVariablesforWeapon _output_get (Variables|Default|GetEquipedWeapon)))

(fn SetAmmunition
  (params (AmmunitionCount :type Integer))
  (bind _equipedweapon (Variables|Default|GetEquipedWeapon))
  (bind _output_get (Variables|/Game/Weapon/BP_MasterWeapon.BP_MasterWeapon_C|SetWeaponStruct _equipedweapon (Utilities|Struct|MakeWeaponStructure (.name (Variables|/Game/Weapon/BP_MasterWeapon.BP_MasterWeapon_C|GetWeaponStruct _equipedweapon)) (.damage (Variables|/Game/Weapon/BP_MasterWeapon.BP_MasterWeapon_C|GetWeaponStruct _equipedweapon)) (.reloadtime (Variables|/Game/Weapon/BP_MasterWeapon.BP_MasterWeapon_C|GetWeaponStruct _equipedweapon)) (.magazinesize (Variables|/Game/Weapon/BP_MasterWeapon.BP_MasterWeapon_C|GetWeaponStruct _equipedweapon)) AmmunitionCount (.weaponclass (Variables|/Game/Weapon/BP_MasterWeapon.BP_MasterWeapon_C|GetWeaponStruct _equipedweapon)) (.shootspeed (Variables|/Game/Weapon/BP_MasterWeapon.BP_MasterWeapon_C|GetWeaponStruct _equipedweapon)) (.singleshoot (Variables|/Game/Weapon/BP_MasterWeapon.BP_MasterWeapon_C|GetWeaponStruct _equipedweapon)))))
  (Default|SetAmmoinMagazine (Variables|Default|GetMagazineWidget) (.ammoinmagazine _output_get)))