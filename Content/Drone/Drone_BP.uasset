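; Drone actor that follows the player and carries out queued tasks, currently build tasks on placeable objects.
; Tasks arrive through an event binding; when idle, Tick picks the highest-priority one, using priority -1 to mean no current task.
; It flies straight toward its target by offsetting its location, then calls StartBuilding on arrival.
; FinishCurrentTask removes the task from the queue and resets it, with no caller in this Blueprint.
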(event Custom|AddTaskToQueue_Event
  (params (NewQueueTask :type Queue%20Task%20Structure))
  (Utilities|Array|Add (Variables|Default|GetTaskQueue) NewQueueTask))

(event EventBeginPlay
  (CallFunction|SetUpDroneVariables)
  (EventDispatchers|BindEventtoAddTasktoQueue (delegate Custom|AddTaskToQueue_Event)))

(event EventTick
  (params (DeltaSeconds :type Float%20%28single-precision%29))
  (bind _currenttaskdescribed (CallFunction|CurrentTaskDescribed))
  (if _currenttaskdescribed
    (CallFunction|ProcessCurerntTask DeltaSeconds)
    (else
      (bind _istaskinqueue (CallFunction|IsTaskinQueue))
      (if _istaskinqueue
        (bind _queuetask (CallFunction|GetTaskfromQueue))
        (bind _output_get (Variables|Default|SetCurrentTask _queuetask))
        (else
          (CallFunction|FollowPlayer DeltaSeconds))))))

(fn ConstructionScript)

(fn FollowPlayer
  (params (delta :type Float%20%28double-precision%29))
  (CallFunction|ApproachActor (Variables|Default|GetPlayer) delta))

(fn SetUpDroneVariables
  (bind _returnvalue (Actor|GetActorOfClass "/Game/ThirdPersonBP/Blueprints/ThirdPersonCharacter.ThirdPersonCharacter_C"))
  (Variables|Default|SetPlayer _returnvalue))

(fn IsTaskinQueue
  (return (> (Utilities|Array|Length (Variables|Default|GetTaskQueue)) 0)))

(fn GetTaskfromQueue
  (bind _taskqueue (Variables|Default|GetTaskQueue))
  (LocalVariables|SetPriorityTask (Utilities|Array|Get(acopy) _taskqueue))
  (for _array_element _taskqueue
    (if (> (.Priority (Utilities|Struct|BreakQueueTask _array_element)) (.priority (LocalVariables|GetPriorityTask)))
      (LocalVariables|SetPriorityTask _array_element)))
  (return (LocalVariables|GetPriorityTask)))

(fn CurrentTaskDescribed
  (return (> (.priority (Variables|Default|GetCurrentTask)) -1)))

(fn ProcessCurerntTask
  (params (delta :type Float%20%28double-precision%29))
  (switch Utilities|FlowControl|Switch|SwitchonTaskType (.tasktype (Variables|Default|GetCurrentTask))
    (:NewEnumerator0
      (CallFunction|ProcessBuildTask (Variables|Default|GetCurrentTask) delta))))

(fn ApproachActor
  (params (Actor :type Actor%20Object%20Reference) (delta :type Float%20%28double-precision%29))
  (bind _returnvalue (Transformation|GetActorLocation))
  (bind _rootcomponent (Variables|/Script/Engine.Actor|GetRootComponent Actor))
  (bind _distancefromdestination (Variables|Default|GetDistanceFromDestination))
  (bind _returnvalue_2 (Transformation|GetWorldLocation _rootcomponent))
  (bind _returnvalue_3 (Math|Vector|Distance(Vector) _returnvalue_2 _returnvalue))
  (bind _returnvalue_4 (<= _returnvalue_3 _distancefromdestination))
  (LocalVariables|SetReachedDestination _returnvalue_4)
  (if _returnvalue_4
    _
    (else
      (Transformation|AddActorWorldOffset (* (* (Math|Vector|Normalize (- _returnvalue_2 _returnvalue)) (Variables|Default|GetFlyingSpeed)) delta))))
  (return (LocalVariables|GetReachedDestination)))

(fn ProcessBuildTask
  (params (Task :type Queue%20Task%20Structure) (delta :type Float%20%28double-precision%29))
  (bind _taskobject (Utilities|Struct|BreakQueueTask Task))
  (if (not (Variables|Default|GetDoingTask))
    (bind _destinationreached (CallFunction|ApproachActor _taskobject delta))
    (if _destinationreached
      (Variables|Default|SetDoingTask true)
      (bind _asplacable_object (Utilities|Casting|CastToPlacableObject _taskobject))
      (Default|StartBuilding _asplacable_object))))

(fn FinishCurrentTask
  (bind _returnvalue (Utilities|Array|RemoveItem (Variables|Default|GetTaskQueue) (Variables|Default|GetCurrentTask)))
  (if _returnvalue
    (CallFunction|SetCurrentTasktoDefault)
    (Variables|Default|SetDoingTask false)
    (else
      (Development|PrintString "Something is wrong and current task is not in task queue"))))

(fn SetCurrentTasktoDefault
  (Variables|Default|SetCurrentTask (Utilities|Struct|MakeQueueTask "NewEnumerator0" 0 -1)))