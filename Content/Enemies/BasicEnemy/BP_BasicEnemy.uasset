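; BP_BasicEnemy is an enemy that heads for the level's objective and reports its death to the wave controller.
; On BeginPlay it uses AIMoveTo toward the first BasicObjective found, printing debug messages.
; Its damage handler subtracts Health and, at zero, calls EnemyKilled on the first WaveController before destroying itself.
; The node binding that handler to OnTakeAnyDamage is disconnected, as are leftover movement-input nodes.
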(event Custom|OnTakeAnyDamage_Event
  (params (DamagedActor :type Actor%20Object%20Reference) (Damage :type Float%20%28single-precision%29) (DamageType :type Damage%20Type%20Object%20Reference) (InstigatedBy :type Controller%20Object%20Reference) (DamageCauser :type Actor%20Object%20Reference))
  ;[1 1 1] Taking damage
  (bind _output_get (Variables|Default|SetHealth (- (Variables|Default|GetHealth) Damage)))
  (if (<= _output_get 0.0)
    (CallFunction|TriggerEnemyKilledEvent)
    (Actor|DestroyActor)))

(event EventBeginPlay
  ;[1 1 1] Start moving to objective
  (bind _outactors (Actor|GetAllActorsOfClass "/Game/Objectives/BasicObjective.BasicObjective_C"))
  (if (== (Utilities|Array|Length _outactors) 0)
    (Development|PrintString "No Objective in the level")
    (else
      (AI|AIMoveTo self "0, 0, 0" (Utilities|Array|Get(acopy) _outactors) 0.5 false
        (:then
          (Development|PrintString "exec"))
        (:OnSuccess
          (Development|PrintString "success"))
        (:OnFail
          (Development|PrintString "Cant find the way to objective"))))))

(fn ConstructionScript)

(fn TriggerEnemyKilledEvent
  (bind _outactors (Actor|GetAllActorsOfClass "/Game/Waves/WaveController.WaveController_C"))
  (if (== (Utilities|Array|Length _outactors) 0)
    (Development|PrintString "No Wave Contorller in the scene")
    (else
      (Default|EnemyKilled (Utilities|Array|Get(acopy) _outactors)))))