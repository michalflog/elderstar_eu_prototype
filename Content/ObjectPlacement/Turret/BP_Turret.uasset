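; Base turret actor for placeable defenses that tracks enemies in range and rate-limits its fire.
; A sphere collision, sized from InRangeRadius on BeginPlay, adds and removes BP_BasicEnemy actors in EnemiesInRange, which helper functions query for presence and the first entry.
; MakeShoot fires the empty Shoot event only when built and ready, then uses a Delay as cooldown.
; Nothing in this graph calls MakeShoot or picks targets automatically.
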(event OnComponentBeginOverlap(InRangeCollision)
  (params (OverlappedComponent :type Primitive%20Component%20Object%20Reference) (OtherActor :type Actor%20Object%20Reference) (OtherComp :type Primitive%20Component%20Object%20Reference) (OtherBodyIndex :type Integer) (bFromSweep :type Boolean) (SweepResult :type Hit%20Result%20Structure%20%28by%20ref%29))
  (CallFunction|AddinRangeEnemy OtherActor))

(event OnComponentEndOverlap(InRangeCollision)
  (params (OverlappedComponent :type Primitive%20Component%20Object%20Reference) (OtherActor :type Actor%20Object%20Reference) (OtherComp :type Primitive%20Component%20Object%20Reference) (OtherBodyIndex :type Integer))
  (CallFunction|RemoveinRangeEnemy OtherActor))

(event Custom|Shoot)

(event Custom|MakeShoot
  (if (and (Variables|Default|GetIsBuild) (Variables|Default|GetCanShoot))
    (Variables|Default|SetCanShoot false)
    (CallFunction|Shoot)
    (Utilities|FlowControl|Delay (Variables|Default|GetShootingInterval))
    (Variables|Default|SetCanShoot true)))

(event EventBeginPlay
  (|CallParentFunction)
  (CallFunction|SetinRangeCollisionRadius))

(event Collision|EventActorBeginOverlap
  (params (OtherActor :type Actor%20Object%20Reference))
  (|CallParentFunction OtherActor) ; This node is disabled and will not be called.\nDrag off pins to build functionality.
)

(event EventTick
  (params (DeltaSeconds :type Float%20%28single-precision%29))
  (|CallParentFunction DeltaSeconds) ; This node is disabled and will not be called.\nDrag off pins to build functionality.
)

(fn ConstructionScript
  (|CallParentFunction))

(fn SetinRangeCollisionRadius
  (Components|Sphere|SetSphereRadius (Variables|Default|GetInRangeCollision) (Variables|Default|GetInRangeRadius) true))

(fn RemoveinRangeEnemy
  (params (Removed%20Actor :type Actor%20Object%20Reference))
  (bind _asbp_basic_enemy (Utilities|Casting|CastToBP_BasicEnemy Removed%20Actor))
  (Utilities|Array|RemoveItem (Variables|Default|GetEnemiesInRange) _asbp_basic_enemy))

(fn AddinRangeEnemy
  (params (AddedActor :type Actor%20Object%20Reference))
  (bind _asbp_basic_enemy (Utilities|Casting|CastToBP_BasicEnemy AddedActor))
  (Utilities|Array|Add (Variables|Default|GetEnemiesInRange) _asbp_basic_enemy))

(fn IsEnemyinRange
  (return (> (Utilities|Array|Length (Variables|Default|GetEnemiesInRange)) 0)))

(fn GetEnemyinRange
  (return (Utilities|Array|Get(acopy) (Variables|Default|GetEnemiesInRange))))