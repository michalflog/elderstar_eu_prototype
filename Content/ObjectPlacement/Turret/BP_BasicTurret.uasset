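; BP_BasicTurret is a placeable turret that fires projectiles, built as a child of a parent turret class.
; Its Shoot override calls the parent logic, then spawns a TurretBullet at the BulletBeginPosition component's transform.
; It then pushes the new bullet along that component's rotation via AddBulletForce.
; The construction script only calls the parent, and the other events are disabled stubs.
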(event EventBeginPlay
  (|CallParentFunction) ; This node is disabled and will not be called.\nDrag off pins to build functionality.
)

(event Collision|EventActorBeginOverlap
  (params (OtherActor :type Actor%20Object%20Reference))
  (|CallParentFunction OtherActor) ; This node is disabled and will not be called.\nDrag off pins to build functionality.
)

(event EventTick
  (params (DeltaSeconds :type Float%20%28single-precision%29))
  (|CallParentFunction DeltaSeconds) ; This node is disabled and will not be called.\nDrag off pins to build functionality.
)

(event EventShoot
  (bind _bulletbeginposition (Variables|Default|GetBulletBeginPosition))
  (|CallParentFunction)
  (bind _returnvalue (Game|SpawnActorfromClass "/Game/Rifles/u-rifle/TurretBullet.TurretBullet_C" (Transformation|GetWorldTransform _bulletbeginposition) "Undefined" 0 (Transformation|GetWorldRotation _bulletbeginposition) 4e+01 0))
  (Default|AddBulletForce _returnvalue (Transformation|GetWorldRotation (Variables|Default|GetBulletBeginPosition))))

(fn ConstructionScript
  (|CallParentFunction))