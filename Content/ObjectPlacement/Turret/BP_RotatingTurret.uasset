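; BP_RotatingTurret is a placeable turret that turns toward an enemy in range and fires at it.
; Each Tick checks for an enemy in range and passes it to RotateToEnemy.
; That function snaps RotatingTuretPart to face the enemy's capsule via look-at rotation, then calls MakeShoot, which defers to the parent.
; The delta time input is unused, and an alternative rotate-until-aligned branch is left disconnected.
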(event EventBeginPlay
  (|CallParentFunction) ; This node is disabled and will not be called.\nDrag off pins to build functionality.
)

(event Collision|EventActorBeginOverlap
  (params (OtherActor :type Actor%20Object%20Reference))
  (|CallParentFunction OtherActor) ; This node is disabled and will not be called.\nDrag off pins to build functionality.
)

(event EventTick
  (params (DeltaSeconds :type Float%20%28single-precision%29))
  (|CallParentFunction DeltaSeconds)
  (bind _isenemyinrange (CallFunction|IsEnemyinRange))
  (if _isenemyinrange
    (bind _enemyinrange (CallFunction|GetEnemyinRange))
    (CallFunction|RotatetoEnemy DeltaSeconds _enemyinrange)))

(event EventMakeShoot
  (|CallParentFunction))

(fn ConstructionScript
  (|CallParentFunction))

(fn RotatetoEnemy
  (params (Delta :type Float%20%28double-precision%29) (Enemy :type BP%20Basic%20Enemy%20Object%20Reference))
  (Transformation|SetWorldRotation (Variables|Default|GetRotatingTuretPart) (Math|Rotator|FindLookatRotation (Transformation|GetWorldLocation (Variables|Default|GetRotatingTuretPart)) (Transformation|GetWorldLocation (Variables|/Script/Engine.Character|GetCapsuleComponent Enemy))) false false)
  (CallFunction|MakeShoot))