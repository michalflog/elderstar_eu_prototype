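; Fire turret Blueprint that extends a parent class and fires projectiles.
; Shoot runs the parent logic, then spawns a TurretBullet at the BulletBeginPosition component and passes that component's world rotation to the bullet's force call.
; Two events toggle TurretCollision between disabled and physics-only through small helper functions.
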(event EventBeginPlay
  (|CallParentFunction) ; This node is disabled and will not be called.\nDrag off pins to build functionality.
)

(event Collision|EventActorBeginOverlap
  (params (OtherActor :type Actor%20Object%20Reference))
  (|CallParentFunction OtherActor) ; This node is disabled and will not be called.\nDrag off pins to build functionality.
)

(event EventTick
  (params (DeltaSeconds :type Float%20%28single-precision%29))
  (|CallParentFunction DeltaSeconds) ; This node is disabled and will not be called.\nDrag off pins to build functionality.
)

(event EventTurnCollisionson
  (CallFunction|Collisionson))

(event EventTurnCollisionsOff
  (CallFunction|CollisionsOff))

(event EventShoot
  (|CallParentFunction)
  (bind _returnvalue (Game|SpawnActorfromClass "/Game/Rifles/u-rifle/TurretBullet.TurretBullet_C" (Transformation|GetWorldTransform (Variables|Default|GetBulletBeginPosition)) "Undefined" 0 "0.000000,0.000000,0.000000" 0))
  (Default|AddBulletForce _returnvalue (Transformation|GetWorldRotation (Variables|Default|GetBulletBeginPosition))))

(fn ConstructionScript
  (|CallParentFunction))

(fn CollisionsOff
  (Collision|SetCollisionEnabled (Variables|Default|GetTurretCollision) "NoCollision"))

(fn Collisionson
  (Collision|SetCollisionEnabled (Variables|Default|GetTurretCollision) "PhysicsOnly"))