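; Placeable spike trap that thrusts its spikes up to damage enemies in its impact area, then retracts and rearms.
; A new overlap, finished building or completed reset triggers it if it is built, ready and has impacted enemies.
; Tick moves the spikes by constant-speed interpolation from the configured up and down times.
; Enemies are damaged when the rise completes, and a delayed reset follows the retraction before retriggering.
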(event Custom|ResetSpike
  (Variables|Default|SetIsGettingReady true)
  (Utilities|FlowControl|Delay (Variables|Default|GetResetTime))
  (Variables|Default|SetIsGettingReady false)
  (Variables|Default|SetReady true)
  (CallFunction|TryDamage))

(event EventBeginPlay
  (|CallParentFunction) ; This node is disabled and will not be called.\nDrag off pins to build functionality.
)

(event Collision|EventActorBeginOverlap
  (params (OtherActor :type Actor%20Object%20Reference))
  (|CallParentFunction OtherActor) ; This node is disabled and will not be called.\nDrag off pins to build functionality.
)

(event EventTick
  (params (DeltaSeconds :type Float%20%28single-precision%29))
  (|CallParentFunction DeltaSeconds)
  (CallFunction|MoveSpike DeltaSeconds))

(event EventOverlapImpactCollision
  (params (OverlapingActor :type Actor%20Object%20Reference))
  (|CallParentFunction OverlapingActor)
  (CallFunction|TryDamage))

(event EventAfterFinishBuilding
  (|CallParentFunction)
  (CallFunction|TryDamage))

(fn ConstructionScript
  (|CallParentFunction))

(fn DamageImpactedEnemies
  (for _array_element (Variables|Default|GetImpactedEnemies)
    (Default|OnTakeAnyDamageEvent _array_element 0 (Variables|Default|GetDamage))))

(fn MoveSpike
  (params (Delta :type Float%20%28double-precision%29))
  (if (not (or (Variables|Default|GetReady) (Variables|Default|GetIsGettingReady)))
    (if (Variables|Default|GetAreSpikesUp)
      (CallFunction|MoveSpikeDown Delta)
      (else
        (CallFunction|MoveSpikeUp Delta)))))

(fn MoveSpikeUp
  (params (Delta :type Float%20%28double-precision%29))
  (bind _spikedownzposition (Variables|Default|GetSpikeDownZPosition))
  (bind _spikeupzposition (Variables|Default|GetSpikeUpZPosition))
  (bind _spikeuptime (Variables|Default|GetSpikeUpTime))
  (bind _spikes (Variables|Default|GetSpikes))
  (bind _spikeupzposition_2 (Variables|Default|GetSpikeUpZPosition))
  (bind _returnvalue (- _spikedownzposition _spikeupzposition))
  (bind _returnvalue_2 (/ 1.0 _spikeuptime))
  (bind _relativelocation (Variables|/Script/Engine.SceneComponent|GetRelativeLocation _spikes))
  (bind _returnvalue_3 (Math|Float|Absolute(Float) _returnvalue))
  (bind _returnvalue_4 (* _returnvalue_3 _returnvalue_2))
  (bind _returnvalue_5 (Math|Interpolation|FInterptoConstant (.z _relativelocation) _spikeupzposition_2 Delta _returnvalue_4))
  (if (>= _returnvalue_5 (Variables|Default|GetSpikeUpZPosition))
    (Variables|Default|SetAreSpikesUp true)
    (CallFunction|DamageImpactedEnemies)
    (else
      (Transformation|SetRelativeLocation (Variables|Default|GetSpikes) (Math|Vector|MakeVector (.x _relativelocation) (.y _relativelocation) _returnvalue_5) false false))))

(fn MoveSpikeDown
  (params (Delta :type Float%20%28double-precision%29))
  (bind _spikedownzposition (Variables|Default|GetSpikeDownZPosition))
  (bind _spikeupzposition (Variables|Default|GetSpikeUpZPosition))
  (bind _spikedowntime (Variables|Default|GetSpikeDownTime))
  (bind _spikedownzposition_2 (Variables|Default|GetSpikeDownZPosition))
  (bind _spikes (Variables|Default|GetSpikes))
  (bind _returnvalue (- _spikedownzposition _spikeupzposition))
  (bind _returnvalue_2 (/ 1.0 _spikedowntime))
  (bind _relativelocation (Variables|/Script/Engine.SceneComponent|GetRelativeLocation _spikes))
  (bind _returnvalue_3 (Math|Float|Absolute(Float) _returnvalue))
  (bind _returnvalue_4 (* _returnvalue_3 _returnvalue_2))
  (bind _returnvalue_5 (Math|Interpolation|FInterptoConstant (.z _relativelocation) _spikedownzposition_2 Delta _returnvalue_4))
  (if (<= _returnvalue_5 (Variables|Default|GetSpikeDownZPosition))
    (Variables|Default|SetAreSpikesUp false)
    (CallFunction|ResetSpike)
    (else
      (Transformation|SetRelativeLocation (Variables|Default|GetSpikes) (Math|Vector|MakeVector (.x _relativelocation) (.y _relativelocation) _returnvalue_5) false false))))

(fn TryDamage
  (if (Math|Boolean|ANDBoolean (> (Utilities|Array|Length (Variables|Default|GetImpactedEnemies)) 0) (Variables|Default|GetReady) (Variables|Default|GetIsBuild))
    (Variables|Default|SetReady false)))