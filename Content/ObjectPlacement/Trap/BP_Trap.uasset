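; BP_Trap is a placeable trap actor that tracks which enemies are inside its impact area.
; ImpactCollision begin and end overlaps add and remove BP_BasicEnemy actors in the ImpactedEnemies collection, ignoring other actor types.
; Begin overlap routes through the OverlapImpactCollision event, while end overlap removes directly.
; The Blueprint itself applies no effect to the tracked enemies.
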(event OnComponentBeginOverlap(ImpactCollision)
  (params (OverlappedComponent :type Primitive%20Component%20Object%20Reference) (OtherActor :type Actor%20Object%20Reference) (OtherComp :type Primitive%20Component%20Object%20Reference) (OtherBodyIndex :type Integer) (bFromSweep :type Boolean) (SweepResult :type Hit%20Result%20Structure%20%28by%20ref%29))
  (CallFunction|OverlapImpactCollision OtherActor))

(event OnComponentEndOverlap(ImpactCollision)
  (params (OverlappedComponent :type Primitive%20Component%20Object%20Reference) (OtherActor :type Actor%20Object%20Reference) (OtherComp :type Primitive%20Component%20Object%20Reference) (OtherBodyIndex :type Integer))
  (CallFunction|RemoveImpactedEnemy OtherActor))

(event Custom|OverlapImpactCollision
  (params (OverlapingActor :type Actor%20Object%20Reference))
  (CallFunction|AddImpactedEnemy OverlapingActor))

(event EventBeginPlay
  (|CallParentFunction) ; This node is disabled and will not be called.\nDrag off pins to build functionality.
)

(event Collision|EventActorBeginOverlap
  (params (OtherActor :type Actor%20Object%20Reference))
  (|CallParentFunction OtherActor) ; This node is disabled and will not be called.\nDrag off pins to build functionality.
)

(event EventTick
  (params (DeltaSeconds :type Float%20%28single-precision%29))
  (|CallParentFunction DeltaSeconds) ; This node is disabled and will not be called.\nDrag off pins to build functionality.
)

(fn ConstructionScript
  (|CallParentFunction))

(fn AddImpactedEnemy
  (params (AddedEnemy :type Actor%20Object%20Reference))
  (bind _asbp_basic_enemy (Utilities|Casting|CastToBP_BasicEnemy AddedEnemy))
  (Utilities|Array|Add (Variables|Default|GetImpactedEnemies) _asbp_basic_enemy))

(fn RemoveImpactedEnemy
  (params (RemovedEnemy :type Actor%20Object%20Reference))
  (bind _asbp_basic_enemy (Utilities|Casting|CastToBP_BasicEnemy RemovedEnemy))
  (Utilities|Array|RemoveItem (Variables|Default|GetImpactedEnemies) _asbp_basic_enemy))